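; Player pawn for a shooter with a shrink mechanic, where shrunk players die when a normal-sized player overlaps them.
; A server event multicasts shrinking or restoring, which drives a timeline that scales the target's capsule and handles collision profile switching.
; Capsule overlaps are checked on authority, applying lethal damage credited to the other character.
; On death, a server event spawns a gun pickup carrying the player's remaining ammo.
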(event OnComponentBeginOverlap(CapsuleComponent)
  (params (OverlappedComponent :type Primitive%20Component%20Object%20Reference) (OtherActor :type Actor%20Object%20Reference) (OtherComp :type Primitive%20Component%20Object%20Reference) (OtherBodyIndex :type Integer) (bFromSweep :type Boolean) (SweepResult :type Hit%20Result%20Structure%20%28by%20ref%29))
  ;[1 1 1] If another non-shrunk player walks on us while we are shrunk, then we die.
  (Networking|SwitchHasAuthority
    (:Authority
      (if (Variables|Default|GetbShrunk)
        (bind _asshooter_character (Utilities|Casting|CastToShooterCharacter OtherActor))
        (if (not (Variables|/Script/ShooterGame.ShooterCharacter|GetbShrunk _asshooter_character))
          (Game|Damage|ApplyDamage self (Variables|Default|GetHealth) (Pawn|GetController _asshooter_character) _asshooter_character "/Script/Engine.DamageType"))))))

(event Custom|ShrinkTarget_Multicast
  (params (Target :type Shooter%20Character%20Object%20Reference) (bReverse :type Boolean))
  (bind _returnvalue (not bReverse))
  (bind _capsulecomponent (Variables|/Script/Engine.Character|GetCapsuleComponent Target))
  ;[1 1 1] Shrink the player or return to normal size based on the Reverse variable.
  (if (and (not (Variables|/Script/ShooterGame.ShooterCharacter|GetbIsDying Target)) _returnvalue)
    (bind _scale (Timeline|ScaleTimeline PlayFromStart)
      (:Update
        (Transformation|SetWorldScale3D _capsulecomponent _scale))
      (:Finished
        (if _returnvalue
          (Collision|SetCollisionProfileName _capsulecomponent "PlayerShrunk" true :!class /Script/Engine.PrimitiveComponent) ; Switch profile to shrunk pawn.
          (else
            (Collision|SetCollisionProfileName _capsulecomponent "PlayerDefault" true :!class /Script/Engine.PrimitiveComponent) ; Restore default profile.
          ))))
    (else
      (Timeline|ScaleTimeline Reverse))))

(event EventServerShrinkEvent
  (params (Target :type Shooter%20Character%20Object%20Reference) (bReverse :type Boolean))
  ;[1 1 1] Run the multicast event.
  (CallFunction|ShrinkTargetMulticast Target bReverse))

(event EventServerCharacterDied
  (params (HeldWeapon :type Shooter%20Weapon%20Class%20Reference) (DeathLocation :type Vector :default "0, 0, 0") (CurrentAmmo :type Integer) (CurrentAmmoInClip :type Integer))
  ;[1 1 1] When a pleyer dies, spawn their weapon as pickup.
  (Game|SpawnActorfromClass "/Game/Blueprints/Pickups/Pickup_Gun.Pickup_Gun_C" (Math|Transform|MakeTransform DeathLocation) "AlwaysSpawn" 0 0 CurrentAmmo CurrentAmmoInClip 0))

(fn ConstructionScript)